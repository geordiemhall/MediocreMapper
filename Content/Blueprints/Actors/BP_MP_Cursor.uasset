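; BP_MP_Cursor is a cursor actor that marks a time position on a note layout with a colored mesh and a name label.
; The construction script runs Init, which pushes Color into the cursor material's Emissive_Color parameter and calls UpdateTransform.
; UpdateTransform places the actor along negative relative Y at Time multiplied by the note separation and refreshes the label from Name.
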(event `init`
  (`MeshComponent.SetVectorParameterValueOnMaterials` (`self.Cursor`) "Emissive_Color" (`self.Color`))
  (`self.UpdateTransform`))

(event `UpdateTransform`
  (`self.K2_SetActorRelativeLocation` (`KismetMathLibrary.MakeVector` 0.0 (* (* (`/Game/Blueprints/BPFL_editor.GetNoteSep`) (`self.Time`)) -1.0)))
  (`TextRenderComponent.K2_SetText` (`self.TextRender`) (`KismetTextLibrary.Conv_StringToText` (`self.Name`))))

(fn `UserConstructionScript`
  (`self.init`))